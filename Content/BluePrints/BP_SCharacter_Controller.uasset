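; BP_SCharacter_Controller is a controller that switches the player between a third-person character and a free "god view" pawn.
; CE_Start spawns BP_SCharacter and a DefaultPawn at given transforms, swaps the pawn's mesh for NULLSM, possesses the character and adds BP_FPP_UI.
; Two custom events swap possession and update the character's view flag.
; Switching to god view first moves the pawn to the character's camera transform.
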(event `self.ReceiveBeginPlay`
  (set `self.IsSCharacterView?` true))

(event `CE_Start`
  (params (StartPoint :type "Transform Structure") (StartTarget :type "Transform Structure"))
  ;[1 1 1] 第三人称视角和上帝视角
  (set `self.StartPoint` StartPoint)
  (set `self.StartTarget` StartTarget)
  (bind _returnvalue (`|SpawnActorFromClass` "/Game/BluePrints/BP_SCharacter.BP_SCharacter_C" (`self.StartPoint`) "Undefined" "OverrideRootScale" null false false true "NewEnumerator0" null))
  (bind _output_get (set `self.SCharacter` _returnvalue))
  (bind _returnvalue_2 (`|SpawnActorFromClass` "/Script/Engine.DefaultPawn" (`self.StartTarget`) "Undefined" "OverrideRootScale" null null))
  (bind _output_get_2 (set `self.DefaultPawn` _returnvalue_2))
  (`StaticMeshComponent.SetStaticMesh` (`DefaultPawn.MeshComponent` _output_get_2) (`self.NULL_SM`))
  (`self.Possess` _output_get)
  (set `self.IsSCharacterView?` true)
  (bind _returnvalue_3 (`|CreateWidget` "/Game/BluePrints/widget/BP_FPP_UI.BP_FPP_UI_C" (`GameplayStatics.GetPlayerController` 0)))
  (`UserWidget.AddToViewport` _returnvalue_3 0))

(event `CE_Change2SCharacter`
  (bind _scharacter (`self.SCharacter`))
  ;[1 1 1] 设置为第三人称视角
  (`self.Possess` _scharacter)
  (set `/Game/BluePrints/BP_SCharacter.IsSCharacterView?` true _scharacter))

(event `CE_Change2DefaultPawn`
  ;[1 1 1] 设置为上帝视角
  (`self.K2_SetActorTransform` (`self.DefaultPawn`) (`SceneComponent.GetSocketTransform` (`SCharacter.CameraComp` (`self.SCharacter`)) "Camera" "RTS_World") false false)
  (`self.Possess` (`self.DefaultPawn`))
  (set `/Game/BluePrints/BP_SCharacter.IsSCharacterView?` false (`self.SCharacter`)))

(fn `UserConstructionScript`)