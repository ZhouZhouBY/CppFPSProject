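; BP_SCharacter is an armed character with mouse-driven firing and touch-drag look controls.
; On BeginPlay it spawns a BP_Weapon, attaches it to the mesh's Weapon socket and stores it.
; Left mouse calls DoFire and Fire, then spawns an explosion particle at FireLoc.
; Touch drags feed pitch and yaw input from the movement since the last touch position, scaled by TurnSpeed and frame time.
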(event `self.ReceiveBeginPlay`
  (bind _returnvalue (`|SpawnActorFromClass` "/Game/BluePrints/BP_Weapon.BP_Weapon_C" (`KismetMathLibrary.MakeTransform` (0.0 0.0 0.0)) "Undefined" "OverrideRootScale" self null))
  (`self.K2_AttachToComponent` _returnvalue (`self.Mesh`) "Weapon" "KeepRelative" "KeepRelative" "KeepRelative" true)
  (set `self.weaponCustom` _returnvalue))

(event `Key|LeftMouseButton`
  (params (Key :type "Key Structure"))
  (:`Pressed`
    (`self.DoFire`)
    (`self.Fire`)
    (`GameplayStatics.SpawnEmitterAtLocation` "/Game/StarterContent/Particles/P_Explosion.P_Explosion" (`self.fireLoc`))))

(event `InputTouch`
  (params (Location :type "Vector Structure") (FingerIndex :type "ETouchIndex Enum"))
  (bind _returnvalue (`GameplayStatics.GetWorldDeltaSeconds`))
  (:`Pressed`
    (set `self.TouchStart` Location))
  (:`Moved`
    (`self.AddControllerPitchInput` (* (.y (- (`self.TouchStart`) Location)) (`self.TurnSpeed`) _returnvalue))
    (`self.AddControllerYawInput` (* (.x (- (`self.TouchStart`) Location)) (`self.TurnSpeed`) _returnvalue))
    (set `self.TouchStart` Location)))

(fn `UserConstructionScript`)