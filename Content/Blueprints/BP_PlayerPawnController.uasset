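; BP_PlayerPawnController is the player's controller, which loads player info at start and handles character respawn requests.
; On BeginPlay it runs its init event, which caches BP_GameInstance and its PlayerInfo, then prints the kill count.
; The rebirth event delegates respawning to BP_GameMode's EVESpawnPlayer, passing itself as the argument.
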(event `self.ReceiveBeginPlay`
  (`self.EVE_Init`))

(event `EVE_Init`
  (bind _asbp_game_instance (cast `/Game/Blueprints/BP_GameInstance` (`GameplayStatics.GetGameInstance`)))
  (bind _output_get (set `self.PlayerInfo` (`/Game/Blueprints/BP_GameInstance.PlayerInfo` _asbp_game_instance)))
  (`KismetSystemLibrary.PrintString` (`KismetStringLibrary.Conv_IntToString` (`.KillNum_5_A4D9FC8744F4B5C8DADCA6A86E48C884` (break `/Game/Blueprints/Str_PlayerInfo` _output_get)))))

(event `EVE_ReBirthCharacter`
  ;[1 1 1] 重新生成玩家角色
  (bind _asbp_game_mode (cast `/Game/Blueprints/BP_GameMode` (`GameplayStatics.GetGameMode`)))
  (`/Game/Blueprints/BP_GameMode.EVE_SpawnPlayer` _asbp_game_mode self))

(fn `UserConstructionScript`)